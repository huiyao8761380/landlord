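; Player controller for Landlord's city view, driving the LLCameraPawn and building placement.
; It moves the pawn by axis input and screen-edge scrolling, scaling axis speed with zoom, and handles spring-arm zoom and gated mouse rotation.
; On BeginPlay it spawns the construction manager and ghost building and creates the city HUD.
; In build mode the ghost follows the cursor; left click queues its construction and removes it, while Deselect cancels.
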(event EventBeginPlay
  (bind _returnvalue (Math|Transform|MakeTransform "0, 0, 0"))
  ;[1 1 1] Init
  (Utilities|FlowControl|Sequence
    (:then_0
      (Utilities|ReferenceCasts))
    (:then_1
      (bind _returnvalue_2 (Game|SpawnActorfromClass "/Game/Landlord/Blueprints/Construction/ConstructionManager_BP.ConstructionManager_BP_C" _returnvalue "AlwaysSpawn" 0 0))
      (Variables|Default|SetConstructionManagerRef _returnvalue_2))
    (:then_2
      (bind _returnvalue_3 (Game|SpawnActorfromClass "/Game/Landlord/Blueprints/Buildings/GhostBuilding_BP.GhostBuilding_BP_C" _returnvalue "AlwaysSpawn" 0 self 0))
      (Variables|Default|SetGhostBuildingRef _returnvalue_3))
    (:then_3
      (Input|SetInputModeGameandUI self 0 "LockAlways" false)
      (Utilities|CreateHUDs)
      (UserInterface|Viewport|AddtoViewport (Variables|Default|GetCityHUDRef) 0))))

(event EventTick
  (params (DeltaSeconds :type Float%20%28single-precision%29))
  (if (Variables|Default|GetIsBuildModeActive)
    (if (!= (Variables|Default|GetGhostBuildingRef) 0)
      (Default|SetCursorWorldPosition (Variables|Default|GetGhostBuildingRef) (CallFunction|SetCursorWorldPosition self (CallFunction|SetSightDistance))))))

(event Input|ActionEvents|InputActionPan
  (params (Key :type Key%20Structure :default "AnyKey"))
  (bind _camerapawnref (Variables|Default|GetCameraPawnRef))
  (bind _returnvalue (Transformation|GetActorRotation _camerapawnref))
  (bind (_roll _pitch _yaw) (Math|Rotator|BreakRotator _returnvalue))
  ;[1 1 1] CameraMovements
  ;;[1 1 1] PanY
  (:Pressed
    (Variables|Default|SetDisableCamNav true)
    (Utilities|FlowControl|Gate true) ; enters at Open
  )
  (:Released
    (Variables|Default|SetDisableCamNav false)
    (Utilities|FlowControl|Gate true) ; enters at Close
  ))

(event Input|ActionEvents|InputActionZoomIn
  (params (Key :type Key%20Structure :default "AnyKey"))
  (bind _camerapawnref (Variables|Default|GetCameraPawnRef))
  (bind _springarm (Variables|/Game/Landlord/Blueprints/LLCameraPawn.LLCameraPawn_C|GetSpringArm _camerapawnref))
  ;[1 1 1] CameraMovements
  ;;[1 1 1] ZoomIn
  (:Pressed
    (Variables|/Script/Engine.SpringArmComponent|SetTargetArmLength _springarm (Math|Float|Clamp(Float) (- (Variables|/Script/Engine.SpringArmComponent|GetTargetArmLength _springarm) (Variables|Default|GetZoomSensitivity)) (Variables|Default|GetMinArmLength) (Variables|Default|GetMaxArmLength)))))

(event Input|ActionEvents|InputActionZoomOut
  (params (Key :type Key%20Structure :default "AnyKey"))
  (bind _camerapawnref (Variables|Default|GetCameraPawnRef))
  (bind _springarm (Variables|/Game/Landlord/Blueprints/LLCameraPawn.LLCameraPawn_C|GetSpringArm _camerapawnref))
  ;[1 1 1] CameraMovements
  ;;[1 1 1] ZoomOut
  (:Pressed
    (Variables|/Script/Engine.SpringArmComponent|SetTargetArmLength _springarm (Math|Float|Clamp(Float) (+ (Variables|/Script/Engine.SpringArmComponent|GetTargetArmLength _springarm) (Variables|Default|GetZoomSensitivity)) (Variables|Default|GetMinArmLength) (Variables|Default|GetMaxArmLength)))))

(event Input|ActionEvents|InputActionPan
  (params (Key :type Key%20Structure :default "AnyKey"))
  (bind _camerapawnref (Variables|Default|GetCameraPawnRef))
  (bind _returnvalue (Transformation|GetActorRotation _camerapawnref))
  (bind (_roll _pitch _yaw) (Math|Rotator|BreakRotator _returnvalue))
  ;[1 1 1] CameraMovements
  ;;[1 1 1] PanX
  (:Pressed
    (Variables|Default|SetDisableCamNav true)
    (Utilities|FlowControl|Gate true) ; enters at Open
  )
  (:Released
    (Variables|Default|SetDisableCamNav false)
    (Utilities|FlowControl|Gate true) ; enters at Close
  ))

(event Input|ActionEvents|InputActionDeselect
  (params (Key :type Key%20Structure :default "AnyKey"))
  (:Pressed
    (if (Variables|Default|GetIsBuildModeActive)
      (Default|KillGhost (Variables|Default|GetGhostBuildingRef)))))

(event Input|ActionEvents|InputActionZoomReset
  (params (Key :type Key%20Structure :default "AnyKey"))
  ;[1 1 1] CameraMovements
  ;;[1 1 1] ZoomReset
  (:Pressed
    (Variables|/Script/Engine.SpringArmComponent|SetTargetArmLength (Variables|/Game/Landlord/Blueprints/LLCameraPawn.LLCameraPawn_C|GetSpringArm (Variables|Default|GetCameraPawnRef)) 1.5e+03)))

(event Input|ActionEvents|InputActionPanReset
  (params (Key :type Key%20Structure :default "AnyKey"))
  (bind _camerapawnref (Variables|Default|GetCameraPawnRef))
  (bind _returnvalue (Transformation|GetActorRotation _camerapawnref))
  (bind (_roll _pitch _yaw) (Math|Rotator|BreakRotator _returnvalue))
  ;[1 1 1] CameraMovements
  ;;[1 1 1] PanReset
  (:Pressed
    (Transformation|SetActorRotation (Variables|Default|GetCameraPawnRef) (Math|Rotator|MakeRotator 0.0 _pitch _yaw))))

(event Input|AxisEvents|InputAxisMoveForward
  (params (AxisValue :type Float%20%28single-precision%29))
  ;[1 1 1] CameraMovements
  ;;[1 1 1] MovementX
  (if (not (Variables|Default|GetDisableCamNav))
    (Transformation|SetActorTransform (Variables|Default|GetCameraPawnRef) (Utilities|MovementX (CallFunction|GetMovementSpeed) (Variables|Default|GetFastMoveMultiplier) AxisValue (Variables|Default|GetCameraPawnRef)))))

(event Input|AxisEvents|InputAxisMoveRight
  (params (AxisValue :type Float%20%28single-precision%29))
  ;[1 1 1] CameraMovements
  ;;[1 1 1] MovementY
  (if (not (Variables|Default|GetDisableCamNav))
    (Transformation|SetActorTransform (Variables|Default|GetCameraPawnRef) (Utilities|MovementY (CallFunction|GetMovementSpeed) (Variables|Default|GetFastMoveMultiplier) AxisValue (Variables|Default|GetCameraPawnRef)))))

(event Input|MouseEvents|MouseX
  (params (AxisValue :type Float%20%28single-precision%29))
  ;[1 1 1] CameraMovements
  ;;[1 1 1] ScreenEdgeMovement
  (if (not (Variables|Default|GetDisableCamNav))
    (bind (_deltaxspeed _deltayspeed) (Utilities|ScreenEdgeMovements))
    (Transformation|AddActorLocalOffset (Variables|Default|GetCameraPawnRef) (Math|Vector|MakeVector _deltaxspeed _deltayspeed 0.0) true false)))

(event Input|MouseEvents|MouseY
  (params (AxisValue :type Float%20%28single-precision%29))
  ;[1 1 1] CameraMovements
  ;;[1 1 1] ScreenEdgeMovement
  (if (not (Variables|Default|GetDisableCamNav))
    (Utilities|ScreenEdgeMovements) ; enters at MouseY
  ))

(event Input|MouseEvents|MouseX
  (params (AxisValue :type Float%20%28single-precision%29))
  (bind _camerapawnref (Variables|Default|GetCameraPawnRef))
  (bind _returnvalue (Transformation|GetActorRotation _camerapawnref))
  (bind (_roll _pitch _yaw) (Math|Rotator|BreakRotator _returnvalue))
  ;[1 1 1] CameraMovements
  ;;[1 1 1] PanX
  (Utilities|FlowControl|Gate true
    (:Exit
      (Transformation|SetActorRotation (Variables|Default|GetCameraPawnRef) (Math|Rotator|MakeRotator _roll _pitch (+ _yaw (* (Variables|Default|GetPanSensitivity) AxisValue)))))))

(event Input|MouseEvents|MouseY
  (params (AxisValue :type Float%20%28single-precision%29))
  (bind _camerapawnref (Variables|Default|GetCameraPawnRef))
  (bind _returnvalue (Transformation|GetActorRotation _camerapawnref))
  (bind (_roll _pitch _yaw) (Math|Rotator|BreakRotator _returnvalue))
  ;[1 1 1] CameraMovements
  ;;[1 1 1] PanY
  (Utilities|FlowControl|Gate true
    (:Exit
      (Transformation|SetActorRotation (Variables|Default|GetCameraPawnRef) (Math|Rotator|MakeRotator _roll (Math|Float|Clamp(Float) (+ _pitch (* (Variables|Default|GetPanSensitivity) AxisValue)) -15.0 45.0) _yaw)))))

(event Input|KeyboardEvents|LeftShift
  (params (Key :type Key%20Structure :default "AnyKey"))
  ;[1 1 1] CameraMovements
  ;;[1 1 1] FastMoveCamera
  (:Pressed
    (Variables|Default|SetFastMoveMultiplier 2.0))
  (:Released
    (Variables|Default|SetFastMoveMultiplier 1.0)))

(event Input|MouseEvents|LeftMouseButton
  (params (Key :type Key%20Structure :default "AnyKey"))
  (:Pressed
    (if (Variables|Default|GetIsBuildModeActive)
      (bind _constructionstruct (Default|GetConstructionStruct (Variables|Default|GetGhostBuildingRef)))
      (Default|QueueConstruction (Variables|Default|GetConstructionManagerRef) _constructionstruct)
      (Default|KillGhost (Variables|Default|GetGhostBuildingRef)))))

(fn ConstructionScript)

(fn GetMovementSpeed
  (bind _camerapawnref (Variables|Default|GetCameraPawnRef))
  (Utilities|IsValid _camerapawnref
    (:Is%20Valid
      (return (Math|Float|Clamp(Float) (/ (Variables|/Script/Engine.SpringArmComponent|GetTargetArmLength (Variables|/Game/Landlord/Blueprints/LLCameraPawn.LLCameraPawn_C|GetSpringArm _camerapawnref)) 1e+02) 5.0 2e+01)))))

(fn SetSightDistance
  (return (+ (Variables|Default|GetSightDistance) (Variables|/Script/Engine.SpringArmComponent|GetTargetArmLength (Variables|/Game/Landlord/Blueprints/LLCameraPawn.LLCameraPawn_C|GetSpringArm (Variables|Default|GetCameraPawnRef))))))

(fn SetCalendar
  (params (Date :type Array%20of%20Integers))
  (return false))

(fn SetClock
  (params (Time :type Array%20of%20Integers))
  (return false))