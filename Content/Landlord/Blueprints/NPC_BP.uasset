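; NPC Blueprint for the Landlord game that randomizes each character's gender, first name and body color.
; The Construction Script calls RandomNPCFeatures, which picks a random gender, then a matching name from male or female name enums via EnumToString.
; A dynamic material instance on the mesh tints BodyColor by gender.
; GetRandomFamilyName exists but is not called here, and the event graph has no active logic.
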(event EventBeginPlay)

(event Collision|EventActorBeginOverlap
  (params (OtherActor :type Actor%20Object%20Reference)))

(event EventTick
  (params (DeltaSeconds :type Float%20%28single-precision%29)))

(fn ConstructionScript
  (CallFunction|RandomNPCFeatures))

(fn RandomNPCFeatures
  (bind _returnvalue (Rendering|Material|CreateDynamicMaterialInstance (Variables|Character|GetMesh) 0 "/Game/Landlord/Mannequin/Character/Materials/M_UE4Man_Body_Inst.M_UE4Man_Body_Inst" :!class /Script/Engine.PrimitiveComponent))
  (LocalVariables|SetMatericalInstance _returnvalue)
  (bind _output_get (LocalVariables|SetGender (Utilities|Enum|ByteToEnumNPC_Gender_ENUM (CallFunction|RandomEnumValue (|GetNumEnumEntries)))))
  (bind _name (CallFunction|GetRandomName _output_get))
  (LocalVariables|SetFirstName _name)
  (switch Utilities|FlowControl|Switch|SwitchonNPC_Gender_ENUM _output_get
    (:NewEnumerator0
      (Rendering|Material|SetVectorParameterValue (LocalVariables|GetMatericalInstance) "BodyColor" (LocalVariables|GetMaleColor) :!class /Script/Engine.MaterialInstanceDynamic))
    (:NewEnumerator1
      (Rendering|Material|SetVectorParameterValue (LocalVariables|GetMatericalInstance) "BodyColor" (LocalVariables|GetFemaleColor) :!class /Script/Engine.MaterialInstanceDynamic))))

(fn GetRandomName
  (params (Gender :type NPC_Gender_ENUM%20Enum))
  (switch Utilities|FlowControl|Switch|SwitchonNPC_Gender_ENUM Gender
    (:NewEnumerator0
      (return (Utilities|String|EnumtoString (CallFunction|GetRandomMaleFirstName))))
    (:NewEnumerator1
      (return (Utilities|String|EnumtoString (CallFunction|GetRandomFemaleFirstName))))))

(fn GetRandomFemaleFirstName
  (return (Utilities|Enum|LiteralenumNPC_Female_Name_ENUM (Utilities|Enum|ByteToEnumNPC_Female_Name_ENUM (CallFunction|RandomEnumValue (|GetNumEnumEntries))))))

(fn GetRandomMaleFirstName
  (return (Utilities|Enum|LiteralenumNPC_Male_Name_ENUM (Utilities|Enum|ByteToEnumNPC_Male_Name_ENUM (CallFunction|RandomEnumValue (|GetNumEnumEntries))))))

(fn GetRandomFamilyName
  (return (Utilities|Enum|LiteralenumNPC_LastNames_ENUM (Utilities|Enum|ByteToEnumNPC_LastNames_ENUM (CallFunction|RandomEnumValue (|GetNumEnumEntries))))))