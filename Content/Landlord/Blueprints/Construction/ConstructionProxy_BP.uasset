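; Construction proxy actor that stands in for a building under construction, showing its display mesh with a ghost material and timing the work.
; It takes the game state's time unit and binds to game speed updates.
; Each tick advances a clockwork value to track time spent against a construction time set from work hours.
; Once done, it calls Construction Completed on every following tick; its delayed self-destroy is unconnected.
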(event Custom|AdjustTime
  (params (TimeUnit :type Float%20%28single-precision%29))
  ;[1 1 1] AdjustTime
  (Variables|Default|SetTimeUnit TimeUnit))

(event EventTick
  (params (DeltaSeconds :type Float%20%28single-precision%29))
  ;[1 1 1] Construction
  (Variables|Default|SetDelta DeltaSeconds)
  (if (Variables|Default|GetIsConstructionCompleted)
    (Default|CallConstructionCompleted self)
    (else
      (CallFunction|DoConstructionWork)
      (Variables|Default|SetIsConstructionCompleted (>= (Variables|Default|GetWorkTimeSpent) (Variables|Default|GetConstructionTime))))))

(event EventBeginPlay
  ;[1 1 1] Init
  (bind _output_get (Variables|References|SetGameStateRef (.AsLLGame%20State (Utilities|Casting|CastToLLGameState (Game|GetGameState)))))
  (Variables|Default|SetTimeUnit (Variables|/Game/Landlord/Blueprints/GameBPS/LLGameState.LLGameState_C|GetTimeUnit _output_get))
  (EventDispatchers|BindEventtoUpdateGameSpeed _output_get (EventDispatchers|CreateEvent :!event Custom|AdjustTime)))

(fn ConstructionScript
  (bind _staticmesh (Variables|Default|GetStaticMesh))
  (Components|StaticMesh|SetStaticMesh _staticmesh (Variables|Default|GetDisplayMesh))
  (Rendering|Material|SetMaterial _staticmesh 0 "/Game/Landlord/Materials/Ghost_M_Construction_Inst.Ghost_M_Construction_Inst"))

(fn SetConstructionTime
  (params (WorkHours :type Float%20%28single-precision%29))
  (bind _output_get (Variables|Default|SetConstructionTime (* WorkHours 6e+01)))
  (return _output_get))

(fn DoConstructionWork
  (bind _output_get (Variables|Default|SetClockwork (.ClockworkOut (CallFunction|SetClockWork (Variables|Default|GetDelta) (Variables|Default|GetTimeUnit) (Variables|Default|GetClockwork)))))
  (Variables|Default|SetWorkTimeSpent (* _output_get 6e+01))
  (return))