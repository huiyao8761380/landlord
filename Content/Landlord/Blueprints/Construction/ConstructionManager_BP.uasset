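; Construction manager Blueprint that queues building projects and swaps temporary construction proxies for the finished buildings.
; QueueConstruction spawns a proxy actor with a display mesh at the target transform, binds its completion event and stores proxy and config in parallel arrays.
; When a proxy reports completion, FinishConstruction finds the matching config by index, removes both entries, spawns the build class at that transform and destroys the proxy.
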(event Custom|BindConstructionComplete
  (params (Proxy :type Construction%20Proxy%20BP%20Object%20Reference))
  (EventDispatchers|BindEventtoConstructionCompleted Proxy (EventDispatchers|CreateEvent :!event Custom|ConstructionCompleted)))

(event Custom|ConstructionCompleted
  (params (Proxy :type Construction%20Proxy%20BP%20Object%20Reference))
  (CallFunction|FinishConstruction Proxy))

(fn ConstructionScript)

(fn QueueConstruction
  (params (ConstructionStruct :type Construction%20Struct%20Structure))
  (bind (_buildclass _proxyclass _transform _displaymesh) (Utilities|Struct|BreakConstructionStruct ConstructionStruct))
  (bind _returnvalue (Game|SpawnActorfromClass _proxyclass _transform "Undefined" 0 _displaymesh 0))
  (CallFunction|BindConstructionComplete _returnvalue)
  (Utilities|Array|Add (Variables|Default|GetProxies) _returnvalue)
  (Utilities|Array|Add (Variables|Default|GetQueue) ConstructionStruct))

(fn FinishConstruction
  (params (Proxy :type Construction%20Proxy%20BP%20Object%20Reference))
  (bind _proxies (Variables|Default|GetProxies))
  (bind _queue (Variables|Default|GetQueue))
  (LocalVariables|Setindex (Utilities|Array|FindItem _proxies Proxy))
  (LocalVariables|SetConfig (Utilities|Array|Get(acopy) _queue (LocalVariables|Getindex)))
  (Utilities|Array|RemoveIndex _queue (LocalVariables|Getindex))
  (Utilities|Array|RemoveIndex _proxies (LocalVariables|Getindex))
  (Game|SpawnActorfromClass (.buildclass (LocalVariables|GetConfig)) (.transform (LocalVariables|GetConfig)) "Undefined" 0 0 0)
  (Actor|DestroyActor Proxy))