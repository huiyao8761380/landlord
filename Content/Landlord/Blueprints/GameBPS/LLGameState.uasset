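; Game state for the Landlord game that runs the in-game clock and calendar and shows both on the city HUD.
; Tick advances an hour-based Clockwork float scaled by TimeUnit, wrapping at 24 to produce a day tick.
; Clock derives hours, minutes and seconds, while Calendar rolls day, month and year, both pushing to the HUD through LLCameraController.
; SetClock and SetCalendar are stubs returning false.
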(event EventBeginPlay
  (bind _asllcamera_controller (Utilities|Casting|CastToLLCameraController (Game|GetPlayerController 0)))
  (Variables|Default|SetControllerRef _asllcamera_controller)
  (Variables|Default|SetClockwork (+ (Math|Conversions|ToFloat(Integer) (Variables|Default|GetSeconds)) (Math|Conversions|ToFloat(Integer) (Variables|Default|GetMinutes)) (Math|Conversions|ToFloat(Integer) (Variables|Default|GetHours))))
  (Variables|Default|SetGameDate (Utilities|Array|MakeArray (Variables|Default|GetDay) (Variables|Default|GetMonth) (Variables|Default|GetYear))))

(event EventTick
  (params (DeltaSeconds :type Float%20%28single-precision%29))
  (bind (_clockwork _daytick) (CallFunction|SetClockwork DeltaSeconds))
  (Variables|Default|SetClockwork _clockwork)
  (Variables|Default|SetDayTick _daytick)
  (CallFunction|Clock)
  (CallFunction|Calendar))

(fn ConstructionScript)

(fn SetClockwork
  (params (DeltaSeconds :type Float%20%28single-precision%29))
  (bind _clockwork (Variables|Default|GetClockwork))
  (bind _timeunit (Variables|Default|GetTimeUnit))
  (bind _returnvalue (/ DeltaSeconds _timeunit))
  (bind _returnvalue_2 (+ _returnvalue _clockwork))
  (bind (_remainder _returnvalue_3) (Math|Float|Division(WholeandRemainder) _returnvalue_2 24.0))
  (return _remainder _returnvalue_3))

(fn Clock
  (bind _clockwork (Variables|Default|GetClockwork))
  (bind _returnvalue (* _clockwork 3.6e+03))
  (bind (_remainder _returnvalue_2) (Math|Float|Division(WholeandRemainder) _returnvalue 6e+01))
  (bind _returnvalue_3 (Math|Conversions|ToFloat(Integer) _returnvalue_2))
  (bind (_remainder_2 _returnvalue_4) (Math|Float|Division(WholeandRemainder) _returnvalue_3 6e+01))
  (Variables|Default|SetSeconds (Math|Float|Floor _remainder))
  (Variables|Default|SetMinutes (Math|Float|Floor _remainder_2))
  (Variables|Default|SetHours (Math|Float|Floor (.Remainder (Math|Float|Division(WholeandRemainder) (Math|Conversions|ToFloat(Integer) _returnvalue_4) 24.0))))
  (bind _output_get (Variables|Default|SetGameTime (Utilities|Array|MakeArray (Variables|Default|GetSeconds) (Variables|Default|GetMinutes) (Variables|Default|GetHours))))
  (Class|ICityViewHUD|SetClock(Message) (Variables|/Game/Landlord/Blueprints/LLCameraController.LLCameraController_C|GetCityHUDRef (Variables|Default|GetControllerRef)) _output_get))

(fn Calendar
  (bind _output_get (Variables|Default|SetDay (+ (Variables|Default|GetDay) (Variables|Default|GetDayTick))))
  (if (> _output_get (Class|KismetMathLibrary|DaysinMonth (Variables|Default|GetYear) (Variables|Default|GetMonth)))
    (Variables|Default|SetDay 1)
    (Variables|Default|SetMonth (+ (Variables|Default|GetMonth) 1)))
  (if (> (Variables|Default|GetMonth) 12)
    (Variables|Default|SetMonth 1)
    (Variables|Default|SetYear (+ (Variables|Default|GetYear) 1)))
  (bind _output_get_2 (Variables|Default|SetGameDate (Utilities|Array|MakeArray (Variables|Default|GetDay) (Variables|Default|GetMonth) (Variables|Default|GetYear))))
  (Class|ICityViewHUD|SetCalendar(Message) (Variables|/Game/Landlord/Blueprints/LLCameraController.LLCameraController_C|GetCityHUDRef (Variables|Default|GetControllerRef)) _output_get_2))

(fn SetCalendar
  (params (Date :type Array%20of%20Integers))
  (return false))

(fn SetClock
  (params (Time :type Array%20of%20Integers))
  (return false))