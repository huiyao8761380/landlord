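; Ghost preview actor for build mode that shows where a building will be placed.
; ConstructBuilding briefly spawns the chosen building to copy its mesh and construction proxy into the ghost, then destroys it.
; While active, a gated Tick snaps the ghost to the grid at the cursor position and swaps to an error material on overlap.
; GetConstructionStruct packages the placement data, and KillGhost clears the preview and exits build mode.
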(event Custom|OnSpawn
  (params (DisplayMesh :type Static%20Mesh%20Object%20Reference) (BuildingClass :type Building%20Master%20BP%20Class%20Reference) (ConstructionProxy :type Construction%20Proxy%20BP%20Class%20Reference))
  ;[1 1 1] OnSpawn
  (if (not (Variables|Default|GetIsActive))
    (Variables|Default|SetBuildingClass BuildingClass)
    (Variables|Default|SetConstructionProxy ConstructionProxy)
    (bind _output_get (Variables|Default|SetDisplayMesh DisplayMesh))
    (Variables|Default|SetIsActive true)
    (Default|SetBuildModeActive (Variables|Default|GetControllerRef) true)
    (Components|StaticMesh|SetStaticMesh (Variables|Default|GetGhostBuilding_Mesh) _output_get)
    (CallFunction|OpenTickGate)
    (CallFunction|SetMaterial (not (CallFunction|CheckOverlap)))))

(event Custom|KillGhost
  ;[1 1 1] KillGhost
  (Variables|Default|SetBuildingClass 0)
  (Variables|Default|SetConstructionProxy 0)
  (CallFunction|CloseTickGate)
  (bind _output_get (Variables|Default|SetDisplayMesh 0))
  (Variables|Default|SetIsActive false)
  (Default|SetBuildModeActive (Variables|Default|GetControllerRef) false)
  (Components|StaticMesh|SetStaticMesh (Variables|Default|GetGhostBuilding_Mesh) _output_get))

(event Custom|OpenTickGate
  ;[1 1 1] FollowMouseCursor
  (Utilities|FlowControl|Gate true) ; enters at Open
)

(event Custom|SetMaterial
  (params (IsErr :type Boolean))
  ;[1 1 1] Set Material
  (if (not (Math|Boolean|Equal(Boolean) IsErr (Variables|Default|GetIsOverlapping)))
    (bind _output_get (Variables|Default|SetIsOverlapping IsErr))
    (if _output_get
      (Rendering|Material|SetMaterial (Variables|Default|GetGhostBuilding_Mesh) 0 "/Game/Landlord/Materials/Ghost_M_Err.Ghost_M_Err")
      (else
        (Rendering|Material|SetMaterial (Variables|Default|GetGhostBuilding_Mesh) 0 "/Game/Landlord/Materials/Ghost_M_Inst.Ghost_M_Inst")))))

(event Custom|CloseTickGate
  ;[1 1 1] FollowMouseCursor
  (Utilities|FlowControl|Gate true) ; enters at Close
)

(event EventConstructBuilding
  (params (Building :type Building%20Master%20BP%20Class%20Reference))
  ;[1 1 1] ConstructBuilding
  (bind _returnvalue (Game|SpawnActorfromClass Building (Math|Transform|MakeTransform "0, 0, 0") "Undefined" 0 (Variables|Default|GetControllerRef) 0))
  (Utilities|FlowControl|Sequence
    (:then_0
      (bind _asbuilding_master_bp (Utilities|Casting|CastToBuildingMaster_BPClass Building))
      (CallFunction|KillGhost)
      (CallFunction|OnSpawn (Variables|/Game/Landlord/Blueprints/Buildings/BuildingMaster_BP.BuildingMaster_BP_C|GetDisplayMesh _returnvalue) _asbuilding_master_bp (Variables|/Game/Landlord/Blueprints/Buildings/BuildingMaster_BP.BuildingMaster_BP_C|GetConstructionProxy _returnvalue)))
    (:then_1
      (Actor|DestroyActor _returnvalue))))

(event EventTick
  (params (DeltaSeconds :type Float%20%28single-precision%29))
  ;[1 1 1] FollowMouseCursor
  (Utilities|FlowControl|Gate true
    (:Exit
      (Transformation|SetActorLocation self (CallFunction|SetSnapGridVector) false false)
      (if (CallFunction|CheckOverlap)
        (CallFunction|SetMaterial true)
        (else
          (CallFunction|SetMaterial false))))))

(fn ConstructionScript)

(fn SetSnapGridVector
  (bind _cursorworldposition (Variables|Default|GetCursorWorldPosition))
  (bind _gridsize (Variables|Default|GetGridSize))
  (bind _returnvalue (Math|Conversions|ToFloat(Integer) _gridsize))
  (return (Math|Vector|MakeVector (Math|Float|SnapToGrid(Float) (.x _cursorworldposition) _returnvalue) (Math|Float|SnapToGrid(Float) (.y _cursorworldposition) _returnvalue) (Math|Float|SnapToGrid(Float) (.z _cursorworldposition) _returnvalue))))

(fn SetCursorWorldPosition
  (params (CursorWorldPosition :type Vector))
  (bind _output_get (Variables|Default|SetCursorWorldPosition CursorWorldPosition))
  (return _output_get))

(fn GetConstructionStruct
  (return (Utilities|Struct|MakeConstructionStruct (Variables|Default|GetBuildingClass) (Variables|Default|GetConstructionProxy) (Math|Transform|MakeTransform (Transformation|GetActorLocation) (Transformation|GetActorRotation)) (Variables|Default|GetDisplayMesh) 1.0)))

(fn CheckOverlap
  (return (> (Utilities|Array|Length (Collision|GetOverlappingActors "/Script/Engine.Actor" :!class /Script/Engine.Actor)) 0)))

(fn SetCalendar
  (params (Date :type Array%20of%20Integers))
  (return false))

(fn SetClock
  (params (Time :type Array%20of%20Integers))
  (return false))